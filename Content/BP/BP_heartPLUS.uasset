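; Heart exchange actor where the player trades 20 pumpkins for one extra life point.
; Overlapping its sphere enables input and a flag, so the Action input can update both counters in BP_ThirdPersonGameMode when enough pumpkins are held.
; Leaving the sphere disables both, and the actor stays for repeat trades.
; On BeginPlay, two randomized timelines animate the yaw of two plank meshes.
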(event OnComponentBeginOverlap(Sphere)
  (params (OverlappedComponent :type Primitive%20Component%20Object%20Reference) (OtherActor :type Actor%20Object%20Reference) (OtherComp :type Primitive%20Component%20Object%20Reference) (OtherBodyIndex :type Integer) (bFromSweep :type Boolean) (SweepResult :type Hit%20Result%20Structure%20%28by%20ref%29))
  (Variables|Default|SetbooleanActionFood true)
  (Input|EnableInput (Game|GetPlayerController 0)))

(event OnComponentEndOverlap(Sphere)
  (params (OverlappedComponent :type Primitive%20Component%20Object%20Reference) (OtherActor :type Actor%20Object%20Reference) (OtherComp :type Primitive%20Component%20Object%20Reference) (OtherBodyIndex :type Integer))
  (Variables|Default|SetbooleanActionFood false)
  (Input|DisableInput (Game|GetPlayerController 0)))

(event EventBeginPlay
  (bind _returnvalue (Math|Random|RandomFloatinRange 0.0 5.0))
  (Utilities|FlowControl|Sequence
    (:then_0
      (bind _rotation (Timeline|Timeline_1 Play)
        (:Update
          (Transformation|SetRelativeRotation (Variables|Default|GetSM_Plank19) (Math|Rotator|MakeRotator 9e+01 0.0 _rotation) false false))))
    (:then_1
      (bind _rotation_2 (Timeline|Timeline_2 Play)
        (:Update
          (Transformation|SetRelativeRotation (Variables|Default|GetSM_Plank18) (Math|Rotator|MakeRotator 9e+01 0.0 _rotation_2) false false))))))

(event Input|ActionEvents|InputActionAction
  (params (Key :type Key%20Structure :default "None"))
  (:Pressed
    (if (Variables|Default|GetbooleanActionFood)
      (bind _asbp_third_person_game_mode (Utilities|Casting|CastToBP_ThirdPersonGameMode (Game|GetGameMode)))
      (if (> (Variables|/Game/ThirdPerson/Blueprints/BP_ThirdPersonGameMode.BP_ThirdPersonGameMode_C|Getpumpkins _asbp_third_person_game_mode) 19)
        (Variables|/Game/ThirdPerson/Blueprints/BP_ThirdPersonGameMode.BP_ThirdPersonGameMode_C|Setpumpkins _asbp_third_person_game_mode (- (Variables|/Game/ThirdPerson/Blueprints/BP_ThirdPersonGameMode.BP_ThirdPersonGameMode_C|Getpumpkins _asbp_third_person_game_mode) 20))
        (Variables|/Game/ThirdPerson/Blueprints/BP_ThirdPersonGameMode.BP_ThirdPersonGameMode_C|SetLIFE%20POINTS _asbp_third_person_game_mode (+ 1 (Variables|/Game/ThirdPerson/Blueprints/BP_ThirdPersonGameMode.BP_ThirdPersonGameMode_C|GetLIFE%20POINTS _asbp_third_person_game_mode)))))))

(fn ConstructionScript)