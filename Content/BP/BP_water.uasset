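; BP_water is a water bucket pickup that the third-person character collects by overlapping its sphere.
; On spawn, timelines scale the bucket and animate its yaw and height, with a randomized timeline time.
; The first valid overlap plays a scale timeline and moves the pickup to the character's Rot component.
; It then destroys itself, plays a sound and spawns a replacement at a random map position.
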(event OnComponentBeginOverlap(Sphere)
  (params (OverlappedComponent :type Primitive%20Component%20Object%20Reference) (OtherActor :type Actor%20Object%20Reference) (OtherComp :type Primitive%20Component%20Object%20Reference) (OtherBodyIndex :type Integer) (bFromSweep :type Boolean) (SweepResult :type Hit%20Result%20Structure%20%28by%20ref%29))
  (bind _asbp_third_person_character (Utilities|Casting|CastToBP_ThirdPersonCharacter OtherActor))
  (Utilities|Casting|CastToBP_ThirdPersonGameMode (Game|GetGameMode))
  (Utilities|FlowControl|DoOnce false
    (:Completed
      (CallFunction|Scale3D)
      (Components|MoveComponentTo (Variables|Default|GetDefaultSceneRoot) (Transformation|GetWorldLocation (Variables|/Game/ThirdPerson/Blueprints/BP_ThirdPersonCharacter.BP_ThirdPersonCharacter_C|Getrot _asbp_third_person_character)) "0, 0, 0" false false 0.2 false)
      (Actor|DestroyActor)
      (Audio|PlaySound2D "/Game/SoulCave/Sound/Cue/Water.Water" 1.0 1.0 0.0 0 0)
      (Game|SpawnActorfromClass "BP_water_C" (Math|Transform|MakeTransform (Math|Vector|MakeVector (Math|Random|RandomFloatinRange -1.3e+02 1.224e+04) (Math|Random|RandomFloatinRange -1577.0 8342.0) 8e+01) "0, 0, 0" "1.000000,1.000000,1.000000") "AdjustIfPossibleButAlwaysSpawn" "MultiplyWithRoot" 0 0))))

(event Custom|Scale3D
  (bind _newtrack_2 (Timeline|Timeline_0 Play)
    (:Update
      (Transformation|SetRelativeScale3D (Variables|Default|GetBusket) (Math|Conversions|ToVector(Float) _newtrack_2)))))

(event EventBeginPlay
  (bind _busket (Variables|Default|GetBusket))
  (Utilities|FlowControl|Sequence
    (:then_0
      (bind _newtrack_2 (Timeline|Timeline_1 Play)
        (:Update
          (Transformation|SetRelativeScale3D (Variables|Default|GetBusket) (Math|Conversions|ToVector(Float) _newtrack_2)))))
    (:then_1
      (Utilities|FlowControl|Sequence
        (:then_0
          (bind (_direction _rotation _location) (Timeline|Timeline Play)
            (:Update
              (Transformation|SetRelativeRotation _busket (Math|Rotator|MakeRotator 0.0 0.0 _rotation) false false)
              (Transformation|SetRelativeLocation _busket (Math|Vector|MakeVector 0.0 0.0 _location) false false))))
        (:then_1
          (Timeline|Timeline SetNewTime))))))

(fn ConstructionScript)

(fn Action)