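; Trigger Blueprint whose Box volume switches seven referenced interactable actors on and off together through activate and deactivate messages.
; Box begin overlap calls ActivateMessage on each ActorInteract reference in turn, and end overlap calls DiactivateMessage on the same set.
; The overlap events do not filter the overlapping actor, and the construction script is empty.
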(event OnComponentBeginOverlap(Box)
  (params (OverlappedComponent :type Primitive%20Component%20Object%20Reference) (OtherActor :type Actor%20Object%20Reference) (OtherComp :type Primitive%20Component%20Object%20Reference) (OtherBodyIndex :type Integer) (bFromSweep :type Boolean) (SweepResult :type Hit%20Result%20Structure%20%28by%20ref%29))
  (Components|Activation|Activate (Variables|Default|Getactor_interact))
  (Components|Activation|Activate (Variables|Default|Getactor_interact_0))
  (Components|Activation|Activate (Variables|Default|Getactor_interact_1))
  (Components|Activation|Activate (Variables|Default|Getactor_interact_2))
  (Components|Activation|Activate (Variables|Default|Getactor_interact_3))
  (Components|Activation|Activate (Variables|Default|Getactor_interact_4))
  (Components|Activation|Activate (Variables|Default|Getactor_interact_5)))

(event OnComponentEndOverlap(Box)
  (params (OverlappedComponent :type Primitive%20Component%20Object%20Reference) (OtherActor :type Actor%20Object%20Reference) (OtherComp :type Primitive%20Component%20Object%20Reference) (OtherBodyIndex :type Integer))
  (Class|Object|Diactivate(Message) (Variables|Default|Getactor_interact))
  (Class|Object|Diactivate(Message) (Variables|Default|Getactor_interact_0))
  (Class|Object|Diactivate(Message) (Variables|Default|Getactor_interact_1))
  (Class|Object|Diactivate(Message) (Variables|Default|Getactor_interact_2))
  (Class|Object|Diactivate(Message) (Variables|Default|Getactor_interact_3))
  (Class|Object|Diactivate(Message) (Variables|Default|Getactor_interact_4))
  (Class|Object|Diactivate(Message) (Variables|Default|Getactor_interact_5)))

(fn ConstructionScript)