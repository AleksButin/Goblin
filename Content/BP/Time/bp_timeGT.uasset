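; Actor that displays elapsed game time as minutes and seconds on its GTMM and GTSS text components.
; Every Tick, TimeSs and TimeMm read game time in seconds and use truncation and integer division to wrap each value by 60.
; The `<= 60` checks let both fields show 60 on the first rollover, and the hours function TimeHh is an empty, uncalled stub.
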(event EventTick
  (params (DeltaSeconds :type Float%20%28single-precision%29))
  (CallFunction|TimeSs)
  (CallFunction|TimeMm))

(fn ConstructionScript)

(fn TimeHh)

(fn TimeMm
  (bind _returnvalue (Utilities|Time|GetGameTimeinSeconds))
  (bind _returnvalue_2 (Math|Float|Truncate _returnvalue))
  (bind _returnvalue_3 (/ _returnvalue_2 60))
  (if (<= _returnvalue_3 60)
    (Rendering|Components|TextRender|SetText (Variables|Default|GetGT_MM) (Utilities|Text|ToText(Integer) _returnvalue_3 false true 2))
    (else
      (Rendering|Components|TextRender|SetText (Variables|Default|GetGT_MM) (Utilities|Text|ToText(Integer) (- _returnvalue_3 (* (/ _returnvalue_3 60) 60)) false true 2)))))

(fn TimeSs
  (bind _returnvalue (Utilities|Time|GetGameTimeinSeconds))
  (bind _gt_ss (Variables|Default|GetGT_SS))
  (bind _returnvalue_2 (Math|Float|Truncate _returnvalue))
  (if (<= _returnvalue_2 60)
    (Rendering|Components|TextRender|SetText _gt_ss (Utilities|Text|ToText(Integer) _returnvalue_2 false true 2))
    (else
      (Rendering|Components|TextRender|SetText _gt_ss (Utilities|Text|ToText(Integer) (- _returnvalue_2 (* (/ _returnvalue_2 60) 60)) false true 2)))))