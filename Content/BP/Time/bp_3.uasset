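; Actor Blueprint that animates a Cube component's relative Z location with a Timeline, starting automatically on BeginPlay.
; Each Timeline update writes the track value to the cube's Z.
; Activate and Diactivate call the PLAY and STOP events to resume or halt the motion, and both always return false.
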(event Custom|STOP
  (bind _newtrack_0 (Timeline|Timeline Stop)
    (:Update
      (Transformation|SetRelativeLocation (Variables|Default|GetCube) (Math|Vector|MakeVector 0.0 0.0 _newtrack_0) false false))))

(event Custom|PLAY
  (bind _newtrack_0 (Timeline|Timeline Play)
    (:Update
      (Transformation|SetRelativeLocation (Variables|Default|GetCube) (Math|Vector|MakeVector 0.0 0.0 _newtrack_0) false false))))

(event EventBeginPlay
  (bind _newtrack_0 (Timeline|Timeline Play)
    (:Update
      (Transformation|SetRelativeLocation (Variables|Default|GetCube) (Math|Vector|MakeVector 0.0 0.0 _newtrack_0) false false))))

(fn ConstructionScript)

(fn Activate
  (CallFunction|PLAY)
  (return false))

(fn Diactivate
  (CallFunction|STOP)
  (return false))