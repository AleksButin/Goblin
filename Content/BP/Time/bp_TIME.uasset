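; An actor that displays two clocks, local real time and elapsed game time, as separate hour, minute and second texts.
; Every tick, RealTime writes the parts of Now as two-digit text.
; GameTime then calls three functions that split truncated game seconds using integer division, without zero padding.
; The minute and hour wrap checks use <=, so exactly 60 minutes or 24 hours display unwrapped.
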(event Custom|RealTime
  (Rendering|Components|TextRender|SetText (Variables|Default|GetRT_HH) (Utilities|Text|ToText(Integer) (Class|KismetMathLibrary|GetHour (Math|DateTime|Now)) false true 2))
  (Rendering|Components|TextRender|SetText (Variables|Default|GetRT_MM) (Utilities|Text|ToText(Integer) (Class|KismetMathLibrary|GetMinute (Math|DateTime|Now)) false true 2 0))
  (Rendering|Components|TextRender|SetText (Variables|Default|GetRT_SS) (Utilities|Text|ToText(Integer) (Class|KismetMathLibrary|GetSecond (Math|DateTime|Now)) false true 2 0)))

(event Custom|GameTime
  (CallFunction|RTSSF)
  (CallFunction|RTMMF)
  (CallFunction|RTHHF))

(event EventTick
  (params (DeltaSeconds :type Float%20%28single-precision%29))
  (CallFunction|RealTime)
  (CallFunction|GameTime))

(fn ConstructionScript)

(fn RTSSF
  (bind _returnvalue (Utilities|Time|GetGameTimeinSeconds))
  (bind _gt_ss (Variables|Default|GetGT_SS))
  (bind _returnvalue_2 (Math|Float|Truncate _returnvalue))
  (if (<= _returnvalue_2 0)
    (Rendering|Components|TextRender|SetText _gt_ss (Utilities|Text|ToText(Integer) _returnvalue_2 false true 2))
    (else
      (Rendering|Components|TextRender|SetText _gt_ss (Utilities|Text|ToText(Integer) (- _returnvalue_2 (* (/ _returnvalue_2 60) 60)) false true 2)))))

(fn RTMMF
  (bind _returnvalue (Utilities|Time|GetGameTimeinSeconds))
  (bind _gt_mm (Variables|Default|GetGT_MM))
  (bind _returnvalue_2 (Math|Float|Truncate _returnvalue))
  (bind _returnvalue_3 (/ _returnvalue_2 60))
  (if (<= _returnvalue_3 60)
    (Rendering|Components|TextRender|SetText _gt_mm (Utilities|Text|ToText(Integer) _returnvalue_3 false true 2))
    (else
      (Rendering|Components|TextRender|SetText _gt_mm (Utilities|Text|ToText(Integer) (- _returnvalue_3 (* (/ _returnvalue_3 60) 60)) false true 2)))))

(fn RTHHF
  (bind _returnvalue (Utilities|Time|GetGameTimeinSeconds))
  (bind _gt_hh (Variables|Default|GetGT_HH))
  (bind _returnvalue_2 (Math|Float|Truncate _returnvalue))
  (bind _returnvalue_3 (/ _returnvalue_2 60))
  (bind _returnvalue_4 (/ _returnvalue_3 60))
  (if (<= _returnvalue_4 24)
    (Rendering|Components|TextRender|SetText _gt_hh (Utilities|Text|ToText(Integer) _returnvalue_4 false true 2))
    (else
      (Rendering|Components|TextRender|SetText _gt_hh (Utilities|Text|ToText(Integer) (- _returnvalue_4 (* (/ _returnvalue_4 24) 24)) false true 2)))))