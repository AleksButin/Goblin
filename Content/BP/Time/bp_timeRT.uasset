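; Actor that displays the current real-world local time as hours, minutes and seconds.
; Every Tick it reads Now, splits out hour, minute and second, and writes each as integer text to its own text component: RTHH, RTMM and RTSS.
; The construction script is empty.
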(event EventTick
  (params (DeltaSeconds :type Float%20%28single-precision%29))
  (Rendering|Components|TextRender|SetText (Variables|Default|GetRT_HH) (Utilities|Text|ToText(Integer) (Class|KismetMathLibrary|GetHour (Math|DateTime|Now)) false true 2 2))
  (Rendering|Components|TextRender|SetText (Variables|Default|GetRT_MM) (Utilities|Text|ToText(Integer) (Class|KismetMathLibrary|GetMinute (Math|DateTime|Now)) false true 2 2))
  (Rendering|Components|TextRender|SetText (Variables|Default|GetRT_SS) (Utilities|Text|ToText(Integer) (Class|KismetMathLibrary|GetSecond (Math|DateTime|Now)) false true 2 2)))

(fn ConstructionScript)