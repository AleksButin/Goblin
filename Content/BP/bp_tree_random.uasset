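; Tree scattering Blueprint that lays out a randomized row of static meshes, presumably trees, along its local Y axis.
; The construction script loops from zero through the Tree count, adding a mesh component each pass with random yaw and uniform scale.
; Each offset is the index times a fresh random spacing, so gaps vary.
; The unseeded layout re-rolls whenever construction reruns, and the event graph is inactive.
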(event EventBeginPlay)

(event Collision|EventActorBeginOverlap
  (params (OtherActor :type Actor%20Object%20Reference)))

(event EventTick
  (params (DeltaSeconds :type Float%20%28single-precision%29)))

(fn ConstructionScript
  (for _index (range 0 (Variables|Default|Gettree))
    (AddComponent|AddStaticMeshComponent false (Math|Transform|MakeTransform (Math|Vector|MakeVector 0.0 (Math|Conversions|ToFloat(Integer) (* _index (Math|Random|RandomIntegerinRange 250 450))) 0.0) (Math|Rotator|MakeRotator 0.0 0.0 (Math|Random|RandomFloatinRange 1e+01 3.5e+02)) (Math|Conversions|ToVector(Float) (Math|Random|RandomFloatinRange 0.6 1.2))))))